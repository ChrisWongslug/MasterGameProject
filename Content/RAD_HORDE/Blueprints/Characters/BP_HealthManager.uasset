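; BP_HealthManager is a health component that tracks a Character owner's health and applies damage to it.
; On BeginPlay the server fills Health from MaxHealth, and the owner is cached as a Character.
; FSApplyDamage subtracts damage and passes the new Health to the owner through IFSetHealthMessage.
; If that call's result is zero or below, it zeroes Health and returns true to signal depletion.
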(event EventBeginPlay
  (Utilities|FlowControl|Sequence
    (:then_0
      (if (Networking|IsServer)
        (Variables|State|SetHealth (Variables|Config|GetMaxHealth))))
    (:then_1
      (bind _ascharacter (Utilities|Casting|CastToCharacter (Components|GetOwner)))
      (Variables|State|SetOwnerCharacter _ascharacter))))

(fn FSApplyDamage
  (params (Damage :type Float%20%28single-precision%29))
  (bind _output_get (Variables|State|SetHealth (- (Variables|State|GetHealth) Damage)))
  (bind _health (Class|BPICharacter|IFSetHealth(Message) (Variables|State|GetOwnerCharacter) _output_get))
  (if (<= _health 0.0)
    (Variables|State|SetHealth 0.0)
    (return true)
    (else
      (return false))))