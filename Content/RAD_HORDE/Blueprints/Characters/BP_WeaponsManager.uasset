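; Character weapon manager that handles a primary (minigun) and secondary (pistol) slot, including shooting input, reloading, switching, adding and dropping.
; Local events gate on busy/reloading flags and call server events, which trigger multicast body and client first-person montages, clearing busy after animation-length delays.
; The server spawns a starting minigun on BeginPlay, and weapons and owner communicate through interface messages.
; A camera line trace also tracks the focusable item being looked at.
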(event Custom|E_EquipSelectedWeapon
  (params (WeaponSlotID :type Integer))
  (bind _item (CallFunction|FGetWeaponbyId WeaponSlotID))
  ;[0 1 0.2061] Equip selected weapon
  (if (not (Variables|State|GetIsBusy))
    (Utilities|IsValid _item :!label _label
      (:Is%20Valid
        (if (not (== _item (Variables|Weapons|GetEquipedWeapon)))
          (Variables|State|SetIsBusy true)
          (CallFunction|EShootReleased)
          (CallFunction|SRVEquipSelectedWeapon WeaponSlotID)
          (bind _asbp_base_character (Utilities|Casting|CastToBP_BaseCharacter (Variables|State|GetOwnerCharacter)))
          (if (Variables|/Game/RAD_HORDE/Blueprints/Characters/BP_BaseCharacter.BP_BaseCharacter_C|GetIsFirstPerson _asbp_base_character)
            _))))
    (elif (Variables|State|GetIsReloading)
      (Variables|State|SetIsBusy false)
      (Variables|State|SetIsReloading false)
      (goto _label))))

(event Custom|E_ShootPressed
  (bind _equipedweapon (Variables|Weapons|GetEquipedWeapon))
  ;[0.8438 0 0.02777] Shot pressed
  (if (not (Variables|State|GetIsBusy))
    (Utilities|IsValid _equipedweapon
      (:Is%20Valid
        (Class|BPIWeapon|IEShotPressed(Message) _equipedweapon)))))

(event Custom|MC_Equip
  ;[1 1 1] Play equip  montage on all clients
  (Animation|PlayAnimMontage (Variables|State|GetOwnerCharacter) (Variables|/Game/RAD_HORDE/Blueprints/Weapons/BP_FirearmWeapon.BP_FirearmWeapon_C|GetCharEquipAnimation (.AsBP%20Firearm%20Weapon (Utilities|Casting|CastToBP_FirearmWeapon (Variables|Weapons|GetEquipedWeapon)))) 1.0 "None"))

(event Custom|MC_Reload
  (bind _ownercharacter (Variables|State|GetOwnerCharacter))
  ;[0.5 0 1] Multicast reload - play animation for all
  (Utilities|IsValid _ownercharacter
    (:Is%20Valid
      (Animation|PlayAnimMontage _ownercharacter (Variables|/Game/RAD_HORDE/Blueprints/Weapons/BP_FirearmWeapon.BP_FirearmWeapon_C|GetCharReloadAnimation (.AsBP%20Firearm%20Weapon (Utilities|Casting|CastToBP_FirearmWeapon (Variables|Weapons|GetEquipedWeapon)))) 1.0 "None"))))

(event Custom|SRV_EquipSelectedWeapon
  (params (WeaponId :type Integer))
  (bind _item (CallFunction|FGetWeaponbyId WeaponId))
  ;[0 1 0.2061] Equip selected weapon
  (Utilities|FlowControl|Sequence
    (:then_0
      (Variables|State|SetWasReloadingAborted (Variables|State|GetIsReloading)))
    (:then_1
      (Variables|State|SetIsBusy true)
      (Utilities|Casting|CastToBP_FirearmWeapon _item)
      (Utilities|FlowControl|Sequence
        (:then_0
          (Utilities|IsValid (Variables|Weapons|GetEquipedWeapon)
            (:Is%20Valid
              (Class|BPIArmedCharacter|IEHolsterWeapon(Message) (Variables|State|GetOwnerCharacter) (Variables|Weapons|GetEquipedWeapon))
              (Variables|Weapons|SetEquipedWeapon 0))))
        (:then_1
          (bind _output_get (Variables|Weapons|SetEquipedWeapon _item))
          (Class|BPIArmedCharacter|IEEquipWeapon(Message) (Variables|State|GetOwnerCharacter) _output_get)
          (CallFunction|MCEquip)
          (CallFunction|CLFPSEquipAnim))
        (:then_2
          (Utilities|FlowControl|Delay (CallFunction|FSGetEquipDelay))
          (Variables|State|SetIsBusy false))))))

(event Custom|E_Reload
  ;[0.5 0 1] Start reloding locally
  (Utilities|FlowControl|Sequence
    (:then_0
      (CallFunction|EShootReleased))
    (:then_1
      (bind _canreload (Class|BPIWeapon|IFCanReload(Message) (Variables|Weapons|GetEquipedWeapon)))
      (if (and _canreload (not (Variables|State|GetIsBusy)))
        (Utilities|IsValid (Variables|Weapons|GetEquipedWeapon)
          (:Is%20Valid
            (Variables|State|SetIsBusy true)
            (CallFunction|SRVReload)
            (bind _asbp_base_character (Utilities|Casting|CastToBP_BaseCharacter (Variables|State|GetOwnerCharacter)))
            (Default|FStopSprint _asbp_base_character))
          (:Is%20Not%20Valid
            (Variables|State|SetIsBusy false)))))))

(event Custom|SRV_Reload
  (bind _equipedweapon (Variables|Weapons|GetEquipedWeapon))
  ;[0.5 0 1] Reload on server
  (Variables|State|SetWasReloadingAborted false)
  (Variables|State|SetIsBusy true)
  (Variables|State|SetIsReloading true)
  (Class|BPIWeapon|IEReload(Message) _equipedweapon)
  (CallFunction|MCReload)
  (CallFunction|CLFPSReloadAnim)
  (Utilities|FlowControl|Delay (- (Variables|/Script/Engine.AnimSequenceBase|GetSequenceLength (Variables|/Game/RAD_HORDE/Blueprints/Weapons/BP_FirearmWeapon.BP_FirearmWeapon_C|GetCharReloadAnimation (.AsBP%20Firearm%20Weapon (Utilities|Casting|CastToBP_FirearmWeapon _equipedweapon)))) 0.1))
  (Variables|State|SetIsBusy false)
  (Variables|State|SetIsReloading false))

(event Custom|E_ScrollWeaponChange
  ;[0 0.0625 0.05657] Change weapon on mouse scroll
  (if (or (not (Variables|State|GetIsBusy)) (Variables|State|GetIsReloading))
    (if (== (Variables|Weapons|GetEquipedWeapon) (Variables|Weapons|GetPrimaryWeapon))
      (CallFunction|EEquipSelectedWeapon 1)
      (else
        (CallFunction|EEquipSelectedWeapon)))))

(event Custom|CL_FPS_EquipAnim
  ;[1 1 1] FPS equip animation
  (bind _asbp_base_character (Utilities|Casting|CastToBP_BaseCharacter (Variables|State|GetOwnerCharacter)))
  (Animation|Montage|MontagePlay (Components|SkeletalMesh|GetAnimInstance (Variables|/Game/RAD_HORDE/Blueprints/Characters/BP_BaseCharacter.BP_BaseCharacter_C|GetFirstPersonSkeletalMesh _asbp_base_character)) "/Game/RAD_HORDE/DemoContent/Animations/FPS/FPP_RifleEquip_Anim_Montage.FPP_RifleEquip_Anim_Montage" 1.0 "MontageLength" 0.0 true))

(event Custom|E_ShootReleased
  (bind _equipedweapon (Variables|Weapons|GetEquipedWeapon))
  ;[0.8438 0 0.02777] Shot released
  (Utilities|IsValid _equipedweapon
    (:Is%20Valid
      (Class|BPIWeapon|IEShotReleased(Message) _equipedweapon))))

(event Custom|CL_FPS_ReloadAnim
  ;[1 1 1] FPS reload animation
  (bind _asbp_base_character (Utilities|Casting|CastToBP_BaseCharacter (Variables|State|GetOwnerCharacter)))
  (Animation|Montage|MontagePlay (Components|SkeletalMesh|GetAnimInstance (Variables|/Game/RAD_HORDE/Blueprints/Characters/BP_BaseCharacter.BP_BaseCharacter_C|GetFirstPersonSkeletalMesh _asbp_base_character)) "/Game/RAD_HORDE/DemoContent/Animations/FPS/FPP_RifleReload_Anim_Montage.FPP_RifleReload_Anim_Montage" 1.0 "MontageLength" 0.0 true))

(event EventBeginPlay
  ;[1 1 1] begin play
  (bind _ascharacter (Utilities|Casting|CastToCharacter (Components|GetOwner)))
  (Variables|State|SetOwnerCharacter _ascharacter)
  (if (Networking|IsServer)
    (WeaponCreation|FSCreateWeaponsatRespawn)))

(fn FGetWeaponbyId
  (params (Id :type Integer))
  (switch int Id
    (:0
      (return (Variables|Weapons|GetPrimaryWeapon)))
    (:1
      (return (Variables|Weapons|GetSecondaryWeapon)))))

(fn FSDestroyAllWeapons
  (Utilities|FlowControl|Sequence
    (:then_0
      (bind _equipedweapon (Variables|Weapons|GetEquipedWeapon)
        (:then
          (Actor|DestroyActor _equipedweapon))
        (:else)))
    (:then_1
      (bind _primaryweapon (Variables|Weapons|GetPrimaryWeapon)
        (:then
          (Actor|DestroyActor _primaryweapon))
        (:else)))
    (:then_2
      (bind _secondaryweapon (Variables|Weapons|GetSecondaryWeapon)
        (:then
          (Actor|DestroyActor _secondaryweapon))
        (:else)))))

(fn FSCreateWeaponsatRespawn
  (bind _weapon (WeaponCreation|FSCreateWeapon "/Game/RAD_HORDE/Blueprints/Weapons/Minigun/BP_Minigun.BP_Minigun_C"))
  (AddingNewWeapon|FSAddNewWeapon _weapon))

(fn FSCreateWeapon
  (params (WeaponClass :type Actor%20Class%20Reference))
  (bind _returnvalue (Game|SpawnActorfromClass WeaponClass (Math|Conversions|ToTransform(Vector) (Transformation|GetSocketLocation (Variables|/Script/Engine.Character|GetMesh (Variables|State|GetOwnerCharacter)) "rhand")) "Undefined" (Variables|State|GetOwnerCharacter) 0))
  (return _returnvalue))

(fn FSAddNewWeapon
  (params (NewWeapon :type Actor%20Object%20Reference))
  (LocalVariables|SetNewWeapon_L NewWeapon)
  (Utilities|FlowControl|Sequence
    (:then_0
      (bind _asbp_firearm_weapon (Utilities|Casting|CastToBP_FirearmWeapon (LocalVariables|GetNewWeapon_L)))
      (Utilities|IsValid (Variables|/Game/RAD_HORDE/Blueprints/Weapons/BP_FirearmWeapon.BP_FirearmWeapon_C|GetOwnerCharacter _asbp_firearm_weapon)
        (:Is%20Not%20Valid
          (Default|FSSetOwner _asbp_firearm_weapon (Variables|State|GetOwnerCharacter)))))
    (:then_1
      (bind _type (Class|BPIWeapon|IFGetWeaponType(Message) (LocalVariables|GetNewWeapon_L)))
      (switch Utilities|FlowControl|Switch|SwitchonE_WeaponType _type
        (:NewEnumerator0
          (Utilities|IsValid (Variables|Weapons|GetPrimaryWeapon)
            (:Is%20Valid
              (if (== (Variables|Weapons|GetEquipedWeapon) (Variables|Weapons|GetPrimaryWeapon))
                (Class|BPIArmedCharacter|IEDropWeapon(Message) (Variables|State|GetOwnerCharacter) (Variables|Weapons|GetPrimaryWeapon))
                (bind _output_get (Variables|Weapons|SetPrimaryWeapon (LocalVariables|GetNewWeapon_L)))
                (bind _output_get_2 (Variables|Weapons|SetEquipedWeapon _output_get))
                (Class|BPIArmedCharacter|IEEquipWeapon(Message) (Variables|State|GetOwnerCharacter) _output_get_2)
                (else
                  (Class|BPIArmedCharacter|IEDropWeapon(Message) (Variables|State|GetOwnerCharacter) (Variables|Weapons|GetPrimaryWeapon))
                  (bind _output_get_3 (Variables|Weapons|SetPrimaryWeapon (LocalVariables|GetNewWeapon_L)))
                  (Class|BPIArmedCharacter|IEHolsterWeapon(Message) (Variables|State|GetOwnerCharacter) _output_get_3))))
            (:Is%20Not%20Valid
              (Variables|Weapons|SetPrimaryWeapon (LocalVariables|GetNewWeapon_L))
              (Utilities|IsValid (Variables|Weapons|GetEquipedWeapon)
                (:Is%20Valid
                  (Class|BPIArmedCharacter|IEHolsterWeapon(Message) (Variables|State|GetOwnerCharacter) (Variables|Weapons|GetPrimaryWeapon)))
                (:Is%20Not%20Valid
                  (bind _output_get_4 (Variables|Weapons|SetEquipedWeapon (Variables|Weapons|GetPrimaryWeapon)))
                  (Class|BPIArmedCharacter|IEEquipWeapon(Message) (Variables|State|GetOwnerCharacter) _output_get_4))))))
        (:NewEnumerator1
          (Utilities|IsValid (Variables|Weapons|GetSecondaryWeapon)
            (:Is%20Valid
              (if (== (Variables|Weapons|GetEquipedWeapon) (Variables|Weapons|GetSecondaryWeapon))
                (Class|BPIArmedCharacter|IEDropWeapon(Message) (Variables|State|GetOwnerCharacter) (Variables|Weapons|GetSecondaryWeapon))
                (bind _output_get_5 (Variables|Weapons|SetSecondaryWeapon (LocalVariables|GetNewWeapon_L)))
                (bind _output_get_6 (Variables|Weapons|SetEquipedWeapon _output_get_5))
                (Class|BPIArmedCharacter|IEEquipWeapon(Message) (Variables|State|GetOwnerCharacter) _output_get_6)
                (else
                  (Class|BPIArmedCharacter|IEDropWeapon(Message) (Variables|State|GetOwnerCharacter) (Variables|Weapons|GetSecondaryWeapon))
                  (bind _output_get_7 (Variables|Weapons|SetSecondaryWeapon (LocalVariables|GetNewWeapon_L)))
                  (Class|BPIArmedCharacter|IEHolsterWeapon(Message) (Variables|State|GetOwnerCharacter) _output_get_7))))
            (:Is%20Not%20Valid
              (Variables|Weapons|SetSecondaryWeapon (LocalVariables|GetNewWeapon_L))
              (Utilities|IsValid (Variables|Weapons|GetEquipedWeapon)
                (:Is%20Valid
                  (Class|BPIArmedCharacter|IEHolsterWeapon(Message) (Variables|State|GetOwnerCharacter) (Variables|Weapons|GetSecondaryWeapon)))
                (:Is%20Not%20Valid
                  (bind _output_get_8 (Variables|Weapons|SetEquipedWeapon (Variables|Weapons|GetSecondaryWeapon)))
                  (Class|BPIArmedCharacter|IEEquipWeapon(Message) (Variables|State|GetOwnerCharacter) _output_get_8))))))))))

(fn FSDropWeapon
  (params (Weapon :type E_WeaponType%20Enum :default "NewEnumerator0"))
  (switch Utilities|FlowControl|Switch|SwitchonE_WeaponType Weapon
    (:NewEnumerator0
      (if (== (Variables|Weapons|GetEquipedWeapon) (Variables|Weapons|GetPrimaryWeapon))
        (Variables|Weapons|SetPrimaryWeapon 0)
        (Variables|Weapons|SetEquipedWeapon 0)
        (Utilities|IsValid (Variables|Weapons|GetSecondaryWeapon)
          (:Is%20Valid
            (CallFunction|SRVEquipSelectedWeapon 1)))
        (else
          (Variables|Weapons|SetPrimaryWeapon 0))))
    (:NewEnumerator1
      (if (== (Variables|Weapons|GetEquipedWeapon) (Variables|Weapons|GetSecondaryWeapon))
        (Variables|Weapons|SetSecondaryWeapon 0)
        (Variables|Weapons|SetEquipedWeapon 0)
        (Utilities|IsValid (Variables|Weapons|GetPrimaryWeapon)
          (:Is%20Valid
            (CallFunction|SRVEquipSelectedWeapon)))
        (else
          (Variables|Weapons|SetSecondaryWeapon 0))))))

(fn FSDropAllWeapons
  (DropWeapons|FSDropWeapon "NewEnumerator0")
  (DropWeapons|FSDropWeapon "NewEnumerator1"))

(fn FSSearchRay
  (bind _camera (Class|BPICharacter|IFGetFollowCamera(Message) (Variables|State|GetOwnerCharacter)))
  (bind (_outhit _returnvalue) (Collision|LineTraceByChannel (Transformation|GetWorldLocation _camera) (+ (Transformation|GetWorldLocation _camera) (* (Math|Vector|GetForwardVector _camera) 5e+02)) "TraceTypeQuery1" false 0 "None"))
  (if _returnvalue
    (bind _canfocus (Class|BPIFocusable|IFCanFocus(Message) (.HitActor (Collision|BreakHitResult _outhit))))
    (if (and _canfocus (Utilities|DoesObjectImplementInterface (.HitActor (Collision|BreakHitResult _outhit)) "/Game/RAD_HORDE/Blueprints/Interfaces/BP_I_Focusable.BP_I_Focusable_C"))
      (if (not (== (Variables|State|GetItemYouAreLookingAt) (.HitActor (Collision|BreakHitResult _outhit))))
        (Variables|State|SetItemYouAreLookingAt (.HitActor (Collision|BreakHitResult _outhit))))
      (else
        (Variables|State|SetItemYouAreLookingAt 0)))
    (else
      (Utilities|IsValid (Variables|State|GetItemYouAreLookingAt)
        (:Is%20Valid
          (Variables|State|SetItemYouAreLookingAt 0))))))

(fn FSGetEquipDelay
  (bind _asbp_base_character (Utilities|Casting|CastToBP_BaseCharacter (Variables|State|GetOwnerCharacter)))
  (if (Variables|/Game/RAD_HORDE/Blueprints/Characters/BP_BaseCharacter.BP_BaseCharacter_C|GetIsFirstPerson _asbp_base_character)
    (return (Variables|/Script/Engine.AnimSequenceBase|GetSequenceLength (Variables|Default|GetFirstPersonEquipAnim)))
    (else
      (bind _asbp_firearm_weapon (Utilities|Casting|CastToBP_FirearmWeapon (Variables|Weapons|GetEquipedWeapon)))
      (return (Variables|/Script/Engine.AnimSequenceBase|GetSequenceLength (Variables|/Game/RAD_HORDE/Blueprints/Weapons/BP_FirearmWeapon.BP_FirearmWeapon_C|GetCharEquipAnimation _asbp_firearm_weapon))))))