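; BP_Minigun_FW is a minigun weapon Blueprint that supplies the muzzle flash effect for the gun.
; FSpawnMuzzleFlash casts the owner to BP_BaseCharacter, then spawns the assault rifle flash emitter at the Minigun mesh's barrel socket transform.
; It branches on whether the owner is player 0 in first person, but both branches currently spawn the identical effect.
; The construction script only calls the parent's.
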(event EventFSpawnMuzzleFlash
  (bind _minigun (Variables|Default|GetMinigun))
  (bind _minigun_2 (Variables|Default|GetMinigun))
  (bind _returnvalue (Transformation|GetSocketTransform _minigun "Barrels_jtSocket" "RTS_World"))
  (bind _returnvalue_2 (Transformation|GetSocketTransform _minigun_2 "Barrels_jtSocket" "RTS_World"))
  (bind _asbp_base_character (Utilities|Casting|CastToBP_BaseCharacter (Variables|Default|GetOwnerCharacter)))
  (if (and (Variables|/Game/RAD_HORDE/Blueprints/Characters/BP_BaseCharacter.BP_BaseCharacter_C|GetIsFirstPerson _asbp_base_character) (== (Game|GetPlayerCharacter 0) (Variables|Default|GetOwnerCharacter)))
    (Effects|SpawnEmitterAttached "/Game/RAD_HORDE/DemoContent/Effects/PS_AssaultRifle_MF.PS_AssaultRifle_MF" 0 "None" (.location _returnvalue_2) (.rotation _returnvalue_2) (.scale _returnvalue_2) "SnapToTargetIncludingScale")
    (else
      (Effects|SpawnEmitterAttached "/Game/RAD_HORDE/DemoContent/Effects/PS_AssaultRifle_MF.PS_AssaultRifle_MF" 0 "None" (.location _returnvalue) (.rotation _returnvalue) (.scale _returnvalue) "SnapToTargetIncludingScale"))))

(fn ConstructionScript
  (|CallParentFunction))