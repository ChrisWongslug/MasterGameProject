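; Horde-mode zombie character that chases living players and bites them, with a random slow or fast walk speed set on the server.
; An AIMoveTo loop targets the last bitten player or a random survivor, then sphere-traces at an arrow to apply damage and multicast the attack montage.
; Depleted health or any headshot kills it, updating kill feed, game state and killer score, then multicasting an impulse-driven ragdoll before timed removal.
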(event Custom|SRV_ChasePlayer
  ;[1 1 1] Chase player
  (bind _movementresult (AI|AIMoveTo self "0, 0, 0" (CallFunction|FSSelectPlayertoChase) 1e+02 false)
    (:OnSuccess
      (switch Utilities|FlowControl|Switch|SwitchonEPathFollowingResult _movementresult
        (:Success
          (AI|Navigation|StopMovement (AI|GetAIController self))
          (CallFunction|EAAttackPlayer))
        (:Blocked
          (Development|PrintString "ai blocked"))
        (:OffPath
          (Development|PrintString "ai off path"))
        (:Aborted
          (Development|PrintString "ai aborted"))
        (:Invalid
          (Development|PrintString "ai invalid"))))
    (:OnFail
      (CallFunction|SRVCHasePlayer))))

(event Custom|MC_Atack
  ;[1 0 0.06864] Multicast attack animation
  (Animation|PlayAnimMontage (Variables|Config|GetAttackAnim) 1.0 "None"))

(event Custom|EA_AttackPlayer
  (bind _arrow1 (Variables|Default|GetArrow1))
  (bind _returnvalue (Transformation|GetWorldLocation _arrow1))
  ;[1 0 0.06749] Attack player
  (bind (_outhit _returnvalue_2) (Collision|SphereTraceByChannel _returnvalue _returnvalue 5e+01 "TraceTypeQuery3" false 0 "None"))
  (if _returnvalue_2
    (bind _asbp_base_character (Utilities|Casting|CastToBP_BaseCharacter (.HitActor (Collision|BreakHitResult _outhit)))
      (:then
        (Game|Damage|ApplyPointDamage _asbp_base_character (Variables|Config|GetDamage) (.Location (Collision|BreakHitResult _outhit)) _outhit)
        (Variables|State|SetLastBittenChar _asbp_base_character)
        (CallFunction|MCAtack)
        (bind _returnvalue_3 (Animation|GetPlayLength (Variables|Config|GetAttackAnim)))
        (Utilities|FlowControl|Delay (+ _returnvalue_3 0.2))
        (CallFunction|SRVCHasePlayer))
      (:CastFailed
        (CallFunction|SRVCHasePlayer :!label _label)))
    (else
      (goto _label))))

(event Custom|MC_Death
  (params (Impulse :type Vector) (Location :type Vector) (LastHitBone :type Name))
  ;[0.7185 1 0] Multicast death by weapon. Apply last shoot  impulse
  (Physics|SetSimulatePhysics (Variables|Character|GetMesh) true)
  (Collision|SetCollisionEnabled (Variables|Collision|GetCapsuleComponent) "NoCollision")
  (Physics|AddImpulseatLocation (Variables|Character|GetMesh) Impulse Location LastHitBone))

(event Game|Damage|EventPointDamage
  (params (Damage :type Float%20%28single-precision%29) (DamageType :type Damage%20Type%20Object%20Reference) (HitLocation :type Vector :default "0, 0, 0") (HitNormal :type Vector :default "0, 0, 0") (HitComponent :type Primitive%20Component%20Object%20Reference) (BoneName :type Name :default "None") (ShotFromDirection :type Vector :default "0, 0, 0") (InstigatedBy :type Controller%20Object%20Reference) (DamageCauser :type Actor%20Object%20Reference) (HitInfo :type Hit%20Result%20Structure%20%28by%20ref%29))
  (bind _returnvalue (Utilities|Name|Equal(Name) BoneName "head"))
  (bind _kernelgs (CallFunction|HKernelGS))
  (bind _returnvalue_2 (Pawn|GetController))
  (bind _playerstate (Variables|/Script/Engine.Controller|GetPlayerState InstigatedBy))
  ;[1 1 1] Apply point damage
  (if (not (Variables|State|GetIsDead))
    (bind _output_get (Variables|State|SetHealth (- (Variables|State|GetHealth) Damage)))
    (if (or (<= _output_get 0.0) _returnvalue)
      (Variables|State|SetIsDead true)
      (Variables|State|SetIsHeadshot _returnvalue)
      (Utilities|FlowControl|Sequence
        (:then_0
          (AI|Navigation|StopMovement _returnvalue_2)
          (Pawn|UnPossess _returnvalue_2))
        (:then_1
          (Default|MCUpdateKillFeed _kernelgs (Variables|/Script/Engine.PlayerState|GetPlayerId _playerstate) (Variables|/Game/RAD_HORDE/Blueprints/Weapons/BP_FirearmWeapon.BP_FirearmWeapon_C|GetWeaponId (.AsBP%20Firearm%20Weapon (Utilities|Casting|CastToBP_FirearmWeapon DamageCauser))) (Variables|State|GetIsHeadshot))
          (Default|EAonZombieDeath _kernelgs))
        (:then_2
          (Class|BPIPlayerStats|IEUpdateKills(Message) _playerstate)
          (if (Variables|State|GetIsHeadshot)
            (Class|BPIPlayerStats|IEUpdateScore(Message) _playerstate (Variables|Config|GetHeadshotScore))
            (else
              (Class|BPIPlayerStats|IEUpdateScore(Message) _playerstate (Variables|Config|GetKillScore)))))
        (:then_3
          (CallFunction|MCDeath (* HitNormal -2e+04) HitLocation BoneName)
          (Actor|SetLifeSpan 5.0))))))

(event EventBeginPlay
  ;[1 1 1] Begin play
  (Utilities|FlowControl|Delay 0.0)
  (Networking|SwitchHasAuthority
    (:Authority
      (Utilities|FlowControl|Sequence
        (:then_0
          ;;[1 1 1] Random - make zombie fast or slow
          (if (Math|Random|RandomBool)
            (Variables|/Script/Engine.CharacterMovementComponent|SetMaxWalkSpeed (Variables|Character|GetCharacterMovement) 2e+02)
            (else
              (Variables|/Script/Engine.CharacterMovementComponent|SetMaxWalkSpeed (Variables|Character|GetCharacterMovement) 375.0))))
        (:then_1
          ;;[1 1 1] Start chasing random player
          (CallFunction|SRVCHasePlayer))))))

(fn ConstructionScript)

(fn FSSelectPlayertoChase
  (bind _aliveplayers (CallFunction|FSGetAlivePlayers))
  (Utilities|IsValid (Variables|State|GetLastBittenChar)
    (:Is%20Valid
      (bind _isdead (Class|BPICharacter|IFIsDead(Message) (Variables|State|GetLastBittenChar)))
      (if (not _isdead)
        (return (Variables|State|GetLastBittenChar))
        (else
          (Variables|State|SetLastBittenChar 0))))
    (:Is%20Not%20Valid
      _))
  (return (Utilities|Array|Get(acopy) _aliveplayers (Math|Random|RandomInteger (Utilities|Array|Length _aliveplayers)))))

(fn FSGetAlivePlayers
  (bind _outactors (Actor|GetAllActorsOfClass "/Game/RAD_HORDE/Blueprints/Characters/BP_BaseCharacter.BP_BaseCharacter_C"))
  (for _array_element _outactors
    (if (not (Variables|/Game/RAD_HORDE/Blueprints/Characters/BP_BaseCharacter.BP_BaseCharacter_C|GetIsDead _array_element))
      (Utilities|Array|AddUnique (LocalVariables|GetAlivePlayers_L) _array_element)))
  (return (LocalVariables|GetAlivePlayers_L)))