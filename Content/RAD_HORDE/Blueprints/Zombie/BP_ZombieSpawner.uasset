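; BP_ZombieSpawner spawns BP_Zombie actors at its location for horde waves up to 8.
; On authority, it binds to the game state's play-time event, which starts a looping timer with a randomized interval.
; The target count scales with wave number; after each spawn and random delay, a level-wide actor count can stop the timer.
; The boss and suicide-grunt count branches are unreachable because their wave checks use AND.
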(event Custom|EA_SpawnZombies
  ;[1 1 1] begin play
  (CallFunction|FSStartSpawnTimer))

(event Custom|EA_SpawnZombie
  (bind _kernelgs (CallFunction|HKernelGS))
  (bind _currentwave (Variables|/Game/RAD_HORDE/Blueprints/Kernel/BP_Kernel_GS.BP_Kernel_GS_C|GetCurrentWave _kernelgs))
  ;[1 1 1] Spawn zombie and stop spawn timer if there are enought zombies
  (Game|SpawnActorfromClass "/Game/RAD_HORDE/Blueprints/Zombie/BP_Zombie.BP_Zombie_C" (Math|Conversions|ToTransform(Vector) (Transformation|GetActorLocation)) "AdjustIfPossibleButAlwaysSpawn" 0 0)
  (Utilities|FlowControl|Delay (Math|Random|RandomFloatinRange 0.0 2.0))
  (if (Math|Boolean|ANDBoolean (== _currentwave 5) (== _currentwave 6) (== _currentwave 7))
    (if (== _currentwave 8)
      (bind _outactors (Actor|GetAllActorsOfClass "/Game/RAD_HORDE/Blueprints/Zombie/BP_Suicide_Grunts.BP_Suicide_Grunts_C"))
      (if (>= (Utilities|Array|Length _outactors) (Variables|Default|GetTotalZombiesAmountToSpawn))
        (Utilities|Time|ClearandInvalidateTimerbyHandle (Variables|Default|GetZombieSpawnTimer)))
      (else
        (bind _outactors_2 (Actor|GetAllActorsOfClass "/Game/RAD_HORDE/Blueprints/Zombie/BP_Boss.BP_Boss_C"))
        (if (>= (Utilities|Array|Length _outactors_2) (Variables|Default|GetTotalZombiesAmountToSpawn))
          (Utilities|Time|ClearandInvalidateTimerbyHandle (Variables|Default|GetZombieSpawnTimer)))))
    (else
      (bind _outactors_3 (Actor|GetAllActorsOfClass "/Game/RAD_HORDE/Blueprints/Zombie/BP_Zombie.BP_Zombie_C"))
      (if (>= (Utilities|Array|Length _outactors_3) (Variables|Default|GetTotalZombiesAmountToSpawn))
        (Utilities|Time|ClearandInvalidateTimerbyHandle (Variables|Default|GetZombieSpawnTimer))))))

(event EventBeginPlay
  (bind _kernelgs (CallFunction|HKernelGS))
  ;[1 1 1] begin play
  (Networking|SwitchHasAuthority
    (:Authority
      (Utilities|IsValid _kernelgs
        (:Is%20Valid
          (EventDispatchers|BindEventtoDPlayTime _kernelgs (delegate Custom|EA_SpawnZombies)))))))

(fn ConstructionScript)

(fn FSStartSpawnTimer
  (bind _kernelgs (CallFunction|HKernelGS))
  (bind _currentwave (Variables|/Game/RAD_HORDE/Blueprints/Kernel/BP_Kernel_GS.BP_Kernel_GS_C|GetCurrentWave _kernelgs))
  (if (< _currentwave 5)
    (Variables|Default|SetTotalZombiesAmountToSpawn (* _currentwave (Variables|Default|GetWaveZombiesAmountToSpawn)) :!label _label)
    (bind _returnvalue (Utilities|Time|SetTimerbyFunctionName 0 "EA_SpawnZombie" (Math|Random|RandomFloatinRange 0.5 2.0) true))
    (Variables|Default|SetZombieSpawnTimer _returnvalue)
    (elif (== _currentwave 5)
      (goto _label)
      (elif (== _currentwave 6)
        (goto _label)
        (elif (== _currentwave 7)
          (goto _label)
          (elif (== _currentwave 8)
            (goto _label)))))))