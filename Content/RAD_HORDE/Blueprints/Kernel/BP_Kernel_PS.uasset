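; Horde-mode player state that tracks each player's kills, deaths, score, money and status.
; On authority it binds to game state dispatchers, resetting stats on the lobby state and awarding score to living players after each wave.
; Interface-style events and getters update and expose the stats, with kills also paying money and team functions left as stubs.
; Score updates trigger a client event that shows a HUD notification and plays a sound.
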(event Custom|E_ResetState
  ;[1 1 1] BEGIN PLAY
  (CallFunction|IEResetStats))

(event Custom|CL_OnScoreUpdate
  (params (Score :type Integer))
  ;[1 1 1] Show notify and play sound on score update
  (Default|FShowScoreNotify (CallFunction|HKernelHUD) (Utilities|String|ToString(Integer) Score))
  (Audio|PlaySound2D "/Game/RAD_HORDE/Sounds/ZombieKillNotifySound_Cue.ZombieKillNotifySound_Cue" 1.0 1.0 0.0 0 0))

(event Custom|EA_UpdateScoreAtWaveCompleted
  ;[1 1 1] BEGIN PLAY
  (if (not (Variables|State|GetIsDead))
    (Playerstats|FSUpdateScore 1000)))

(event EventBeginPlay
  (bind _kernelgs (CallFunction|HKernelGS))
  ;[1 1 1] BEGIN PLAY
  (Networking|SwitchHasAuthority
    (:Authority
      (EventDispatchers|BindEventtoDLobbyState _kernelgs (delegate Custom|E_ResetState))
      (EventDispatchers|BindEventtoDAfterWave _kernelgs (delegate Custom|EA_UpdateScoreAtWaveCompleted)))))

(event EventIEUpdateKills
  ;[1 1 1] Update kills and add money
  (Playerstats|FSIncrementKills)
  (Playerstats|FSAddMoney 100))

(event EventIEUpdateScore
  (params (AddScore :type Integer))
  ;[1 1 1] Update score
  (Playerstats|FSUpdateScore AddScore)
  (CallFunction|CLonScoreUpdate AddScore))

(event EventIEUpdateDeaths
  ;[1 1 1] Update deaths
  (Playerstats|FSIncrementDeaths))

(event EventIEResetStats
  ;[1 1 1] Reset all stats
  (Variables|State|SetKills 0)
  (Variables|State|SetDeaths 0)
  (Variables|State|SetMyScore 0)
  (Variables|State|SetIsDead false)
  (Variables|State|SetIsReady false)
  (Variables|State|SetHealth 1e+02)
  (Variables|State|SetMoney 0))

(fn ConstructionScript)

(fn FSIncrementKills
  (bind _output_get (Variables|State|SetKills (+ (Variables|State|GetKills) 1)))
  (return _output_get))

(fn FSIncrementDeaths
  (bind _output_get (Variables|State|SetDeaths (+ (Variables|State|GetDeaths) 1)))
  (return _output_get))

(fn FSUpdateScore
  (params (AddScore :type Integer))
  (Variables|State|SetMyScore (+ AddScore (Variables|State|GetMyScore)))
  (return 0))

(fn FSAddMoney
  (params (Add :type Integer))
  (Variables|State|SetMoney (+ Add (Variables|State|GetMoney)))
  (return 0))

(fn IFGetDeaths
  (return (Variables|State|GetDeaths)))

(fn IFGetKills
  (return (Variables|State|GetKills)))

(fn IFGetScore
  (return (Variables|State|GetMyScore)))

(fn IFGetTeam
  (return 0))

(fn IFSetTeam
  (params (NewTeam :type Integer)))