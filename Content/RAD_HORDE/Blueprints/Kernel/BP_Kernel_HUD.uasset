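; Horde-mode HUD that owns the player's UI widgets, from lobby and loading screen to in-game HUD, kill feed, chat and match finish.
; On BeginPlay it binds to kernel game state events, which clear most screens and show those for the new phase.
; Kill, chat and wave-completion events add messages or notifications.
; Toggle functions lazily create and cache widgets, also covering menu, scoreboard, help, bleeding and observer overlays.
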(event Custom|E_OnMatchStart
  (bind _returnvalue (Game|GetPlayerController 0))
  ;[1 1 1] Show player hud and kill feed at match start
  (Variables|/Script/Engine.PlayerController|SetbShowMouseCursor _returnvalue false)
  (Input|SetInputModeGameOnly _returnvalue)
  (WidgetRemoving|FRemoveAll)
  (MainWidgets|FTogglePlayerHud true)
  (MainWidgets|FToggleKillFeed true))

(event Custom|E_UpdateKillsLog
  (params (PlayerId :type Integer) (WeaponId :type Integer) (IsHeadShot :type Boolean))
  ;[1 1 1] Update kills log
  (Utilities|IsValid (Variables|WidgetsRefs|GetKillFeed)
    (:Is%20Valid
      (bind _returnvalue (UserInterface|CreateWidget "/Game/RAD_HORDE/Blueprints/Widgets/Game/BP_WE_KillFeedMessage.BP_WE_KillFeedMessage_C" (Variables|Default|GetPlayerOwner) PlayerId WeaponId IsHeadShot))
      (Default|EAddMessage (Variables|WidgetsRefs|GetKillFeed) _returnvalue))))

(event Custom|E_OnLobbyState
  ;[1 1 1] show lobby
  (WidgetRemoving|FRemoveAll)
  (MainWidgets|FToggleLobby true)
  (Variables|/Script/Engine.PlayerController|SetbShowMouseCursor (Game|GetPlayerController 0) true))

(event Custom|E_OnWaveCompleted
  ;[1 1 1] On wave completed
  (Notify|FShowWaveSurviveNotify))

(event Custom|E_ShowHitIndicator
  (bind _playerhud (Variables|WidgetsRefs|GetPlayerHud))
  ;[1 0 0.2682] Show and slowly hide enemy hit indicator
  (Utilities|IsValid _playerhud
    (:Is%20Valid
      (Default|EActivateHitIndicator _playerhud))))

(event Custom|E_UpdateLobbyChat
  (params (PlayerId :type Integer) (Message :type String))
  ;[1 1 1] Update lobby chat
  (Default|EAddLobbyMessage (Variables|WidgetsRefs|GetLobby) PlayerId Message))

(event Custom|E_OnGameStartDelay
  ;[1 1 1] Show loading screen
  (WidgetRemoving|FRemoveAll)
  (MainWidgets|FToggleLoadingScreen true))

(event Custom|E_OnMatchFinish
  ;[1 1 1] Show match finish widget with winner name
  (WidgetRemoving|FRemoveAll)
  (MainWidgets|FToggleMatchFinishScreen true))

(event Custom|E_UpdateGameChat
  (params (IsServer :type Boolean) (SenderId :type Integer) (Message :type String))
  ;[1 1 1] Update game chat
  (UserCalledWidgets|FToggleGameChat true)
  (Default|EAddMessage (Variables|WidgetsRefs|GetGameChat) IsServer SenderId Message))

(event EventBeginPlay
  (MainWidgets|FToggleLoadingScreen true)
  (Utilities|IsValid (Game|GetGameState)
    (:Is%20Valid
      _)
    (:Is%20Not%20Valid
      (Utilities|FlowControl|Delay 1.0)))
  (Utilities|FlowControl|Sequence
    (:then_0
      ;[1 1 1] Define what widget to show on begin play
      (switch Utilities|FlowControl|Switch|SwitchonE_GlobalState (Variables|/Game/RAD_HORDE/Blueprints/Kernel/BP_Kernel_GS.BP_Kernel_GS_C|GetGlobalState (CallFunction|HKernelGS))
        (:NewEnumerator0
          (WidgetRemoving|FRemoveAll)
          (MainWidgets|FToggleLobby true))
        (:NewEnumerator26
          (WidgetRemoving|FRemoveAll)
          (MainWidgets|FToggleMatchFinishScreen true))))
    (:then_1
      ;[1 1 1] Show loading screen
      (EventDispatchers|BindEventtoDGameStartDelay (CallFunction|HKernelGS) (delegate Custom|E_OnGameStartDelay)))
    (:then_2
      ;[1 1 1] show lobby
      (EventDispatchers|BindEventtoDLobbyState (CallFunction|HKernelGS) (delegate Custom|E_OnLobbyState))
      ;[1 1 1] On wave completed
      (EventDispatchers|BindEventtoDAfterWave (CallFunction|HKernelGS) (delegate Custom|E_OnWaveCompleted)))
    (:then_3
      ;[1 1 1] Show player hud and kill feed at match start
      (EventDispatchers|BindEventtoDMatchStart (CallFunction|HKernelGS) (delegate Custom|E_OnMatchStart)))
    (:then_4
      ;[1 1 1] Show match finish widget with winner name
      (EventDispatchers|BindEventtoDMatchFinish (CallFunction|HKernelGS) (delegate Custom|E_OnMatchFinish)))
    (:then_5
      ;[1 1 1] Update kills log
      (EventDispatchers|BindEventtoDUpdateKillFeed (CallFunction|HKernelGS) (delegate Custom|E_UpdateKillsLog)))
    (:then_6
      ;[1 1 1] Update game chat
      (EventDispatchers|BindEventtoDUpdateGameChat (CallFunction|HKernelGS) (delegate Custom|E_UpdateGameChat)))
    (:then_7
      ;[1 1 1] Update lobby chat
      (EventDispatchers|BindEventtoDUpdateLobbyChat (CallFunction|HKernelGS) (delegate Custom|E_UpdateLobbyChat)))))

(fn ConstructionScript)

(fn FTogglePlayerHud
  (params (Show :type Boolean))
  (if Show
    (Variables|WidgetsRefs|GetPlayerHud
      (:then
        (Utilities|MHIsWidgetVisible (Variables|WidgetsRefs|GetPlayerHud)
          (:false
            (UserInterface|Viewport|AddtoViewport (Variables|WidgetsRefs|GetPlayerHud) 0))))
      (:else
        (bind _returnvalue (UserInterface|CreateWidget "/Game/RAD_HORDE/Blueprints/Widgets/Game/BP_W_HUD.BP_W_HUD_C" (Variables|Default|GetPlayerOwner)))
        (bind _output_get (Variables|WidgetsRefs|SetPlayerHud _returnvalue))
        (UserInterface|Viewport|AddtoViewport _output_get 0)))
    (else
      (bind _playerhud (Variables|WidgetsRefs|GetPlayerHud)
        (:then
          (Widget|RemovefromParent _playerhud))
        (:else)))))

(fn FToggleKillFeed
  (params (Show :type Boolean))
  (if Show
    (Variables|WidgetsRefs|GetKillFeed
      (:then
        (Utilities|MHIsWidgetVisible (Variables|WidgetsRefs|GetKillFeed)
          (:false
            (UserInterface|Viewport|AddtoViewport (Variables|WidgetsRefs|GetKillFeed) 0))))
      (:else
        (bind _returnvalue (UserInterface|CreateWidget "/Game/RAD_HORDE/Blueprints/Widgets/Game/BP_W_KillFeed.BP_W_KillFeed_C" (Variables|Default|GetPlayerOwner)))
        (bind _output_get (Variables|WidgetsRefs|SetKillFeed _returnvalue))
        (UserInterface|Viewport|AddtoViewport _output_get 0)))
    (else
      (bind _killfeed (Variables|WidgetsRefs|GetKillFeed)
        (:then
          (Widget|RemovefromParent _killfeed))
        (:else)))))

(fn FToggleinGameMenu
  (params (Show :type Boolean))
  (if Show
    (Variables|WidgetsRefs|GetInGameMenu
      (:then
        (Utilities|MHIsWidgetVisible (Variables|WidgetsRefs|GetInGameMenu)
          (:false
            (UserInterface|Viewport|AddtoViewport (Variables|WidgetsRefs|GetInGameMenu) 99))))
      (:else
        (bind _returnvalue (UserInterface|CreateWidget "/Game/RAD_HORDE/Blueprints/Widgets/Game/BP_W_InGameMenu.BP_W_InGameMenu_C" (Variables|Default|GetPlayerOwner)))
        (bind _output_get (Variables|WidgetsRefs|SetInGameMenu _returnvalue))
        (UserInterface|Viewport|AddtoViewport _output_get 99)))
    (else
      (bind _ingamemenu (Variables|WidgetsRefs|GetInGameMenu)
        (:then
          (Widget|RemovefromParent _ingamemenu))
        (:else)))))

(fn FToggleMatchFinishScreen
  (params (Show :type Boolean))
  (if Show
    (Variables|WidgetsRefs|GetMatchFinishScreen
      (:then
        (Utilities|MHIsWidgetVisible (Variables|WidgetsRefs|GetMatchFinishScreen)
          (:false
            (UserInterface|Viewport|AddtoViewport (Variables|WidgetsRefs|GetMatchFinishScreen) 0))))
      (:else
        (bind _returnvalue (UserInterface|CreateWidget "/Game/RAD_HORDE/Blueprints/Widgets/Game/BP_W_MatchFinishScreen.BP_W_MatchFinishScreen_C" (Variables|Default|GetPlayerOwner)))
        (bind _output_get (Variables|WidgetsRefs|SetMatchFinishScreen _returnvalue))
        (UserInterface|Viewport|AddtoViewport _output_get 0)))
    (else
      (bind _matchfinishscreen (Variables|WidgetsRefs|GetMatchFinishScreen)
        (:then
          (Widget|RemovefromParent _matchfinishscreen))
        (:else)))))

(fn FRemoveAll
  (Utilities|FlowControl|Sequence
    (:then_0
      (bind _playerhud (Variables|WidgetsRefs|GetPlayerHud)
        (:then
          (Widget|RemovefromParent _playerhud)
          (Variables|WidgetsRefs|SetPlayerHud 0))
        (:else)))
    (:then_1
      (bind _killfeed (Variables|WidgetsRefs|GetKillFeed)
        (:then
          (Widget|RemovefromParent _killfeed)
          (Variables|WidgetsRefs|SetKillFeed 0))
        (:else)))
    (:then_2
      (bind _matchfinishscreen (Variables|WidgetsRefs|GetMatchFinishScreen)
        (:then
          (Widget|RemovefromParent _matchfinishscreen)
          (Variables|WidgetsRefs|SetMatchFinishScreen 0))
        (:else)))
    (:then_3
      (bind _killfeed_2 (Variables|WidgetsRefs|GetKillFeed)
        (:then
          (Widget|RemovefromParent _killfeed_2)
          (Variables|WidgetsRefs|SetKillFeed 0))
        (:else)))
    (:then_4
      (bind _lobby (Variables|WidgetsRefs|GetLobby)
        (:then
          (Widget|RemovefromParent _lobby)
          (Variables|WidgetsRefs|SetLobby 0))
        (:else)))
    (:then_5
      (bind _observerhud (Variables|WidgetsRefs|GetObserverHud)
        (:then
          (Widget|RemovefromParent _observerhud)
          (Variables|WidgetsRefs|SetObserverHud 0))
        (:else)))
    (:then_6
      (bind _bleedingscreen (Variables|WidgetsRefs|GetBleedingScreen)
        (:then
          (Widget|RemovefromParent _bleedingscreen)
          (Variables|WidgetsRefs|SetBleedingScreen 0))
        (:else)))))

(fn FToggleLobby
  (params (Show :type Boolean))
  (if Show
    (Variables|WidgetsRefs|GetLobby
      (:then
        (Utilities|MHIsWidgetVisible (Variables|WidgetsRefs|GetLobby)
          (:false
            (UserInterface|Viewport|AddtoViewport (Variables|WidgetsRefs|GetLobby) 0))))
      (:else
        (bind _returnvalue (UserInterface|CreateWidget "/Game/RAD_HORDE/Blueprints/Widgets/Lobby/BP_W_Lobby.BP_W_Lobby_C" (Variables|Default|GetPlayerOwner)))
        (bind _output_get (Variables|WidgetsRefs|SetLobby _returnvalue))
        (UserInterface|Viewport|AddtoViewport _output_get 0)))
    (else
      (bind _lobby (Variables|WidgetsRefs|GetLobby)
        (:then
          (Widget|RemovefromParent _lobby))
        (:else)))))

(fn FToggleLoadingScreen
  (params (Show :type Boolean))
  (if Show
    (Variables|WidgetsRefs|GetLoadingScreen
      (:then
        (Utilities|MHIsWidgetVisible (Variables|WidgetsRefs|GetLoadingScreen)
          (:false
            (UserInterface|Viewport|AddtoViewport (Variables|WidgetsRefs|GetLoadingScreen) 0))))
      (:else
        (bind _returnvalue (UserInterface|CreateWidget "/Game/RAD_HORDE/Blueprints/Widgets/Game/BP_W_LoadingScreen.BP_W_LoadingScreen_C" (Variables|Default|GetPlayerOwner) (Math|Conversions|ToFloat(Integer) (Variables|/Game/RAD_HORDE/Blueprints/Kernel/BP_Kernel_GS.BP_Kernel_GS_C|GetGameStartDelayS (CallFunction|HKernelGS)))))
        (bind _output_get (Variables|WidgetsRefs|SetLoadingScreen _returnvalue))
        (UserInterface|Viewport|AddtoViewport _output_get 0)))
    (else
      (bind _loadingscreen (Variables|WidgetsRefs|GetLoadingScreen)
        (:then
          (Widget|RemovefromParent _loadingscreen))
        (:else)))))

(fn FShowScoreNotify
  (params (Score :type String))
  (Utilities|FlowControl|Sequence
    (:then_0
      (bind _scorenotify (Variables|WidgetsRefs|GetScoreNotify)
        (:then
          (Widget|RemovefromParent _scorenotify))
        (:else)))
    (:then_1
      (bind _returnvalue (UserInterface|CreateWidget "/Game/RAD_HORDE/Blueprints/Widgets/Game/BP_W_ScoreNotify.BP_W_ScoreNotify_C" (Variables|Default|GetPlayerOwner) Score))
      (bind _output_get (Variables|WidgetsRefs|SetScoreNotify _returnvalue))
      (UserInterface|Viewport|AddtoViewport _output_get 0))))

(fn FToggleGameChat
  (params (Show :type Boolean))
  (if Show
    (Variables|WidgetsRefs|GetGameChat
      (:then
        (Utilities|MHIsWidgetVisible (Variables|WidgetsRefs|GetGameChat)
          (:false
            (UserInterface|Viewport|AddtoViewport (Variables|WidgetsRefs|GetGameChat) 100))))
      (:else
        (bind _returnvalue (UserInterface|CreateWidget "/Game/RAD_HORDE/Blueprints/Widgets/Chat/BP_W_GameChat.BP_W_GameChat_C" (Variables|Default|GetPlayerOwner)))
        (bind _output_get (Variables|WidgetsRefs|SetGameChat _returnvalue))
        (UserInterface|Viewport|AddtoViewport _output_get 100)))
    (else
      (bind _gamechat (Variables|WidgetsRefs|GetGameChat)
        (:then
          (Widget|RemovefromParent _gamechat))
        (:else)))))

(fn FToggleScoreboard
  (params (Show :type Boolean))
  (if Show
    (Variables|WidgetsRefs|GetScoreboard
      (:then
        (Utilities|MHIsWidgetVisible (Variables|WidgetsRefs|GetScoreboard)
          (:false
            (UserInterface|Viewport|AddtoViewport (Variables|WidgetsRefs|GetScoreboard) 100))))
      (:else
        (bind _returnvalue (UserInterface|CreateWidget "/Game/RAD_HORDE/Blueprints/Widgets/Scoreboard/BP_W_ScoreBoard.BP_W_ScoreBoard_C" (Variables|Default|GetPlayerOwner)))
        (bind _output_get (Variables|WidgetsRefs|SetScoreboard _returnvalue))
        (UserInterface|Viewport|AddtoViewport _output_get 100)))
    (else
      (bind _scoreboard (Variables|WidgetsRefs|GetScoreboard)
        (:then
          (Widget|RemovefromParent _scoreboard))
        (:else)))))

(fn FToggleHelp
  (params (Show :type Boolean))
  (if Show
    (Variables|WidgetsRefs|GetHelp
      (:then
        (Utilities|MHIsWidgetVisible (Variables|WidgetsRefs|GetHelp)
          (:false
            (UserInterface|Viewport|AddtoViewport (Variables|WidgetsRefs|GetHelp) 100))))
      (:else
        (bind _returnvalue (UserInterface|CreateWidget "/Game/RAD_HORDE/Blueprints/Widgets/Game/BP_W_Help.BP_W_Help_C" (Variables|Default|GetPlayerOwner)))
        (bind _output_get (Variables|WidgetsRefs|SetHelp _returnvalue))
        (UserInterface|Viewport|AddtoViewport _output_get 100)))
    (else
      (bind _help (Variables|WidgetsRefs|GetHelp)
        (:then
          (Widget|RemovefromParent _help))
        (:else)))))

(fn FShowWaveSurviveNotify
  (bind _returnvalue (UserInterface|CreateWidget "/Game/RAD_HORDE/Blueprints/Widgets/Game/BP_W_WaveSurviveNotify.BP_W_WaveSurviveNotify_C" (Variables|Default|GetPlayerOwner)))
  (UserInterface|Viewport|AddtoViewport _returnvalue 0))

(fn FToggleBleedingScreen
  (params (Show :type Boolean))
  (if Show
    (Variables|WidgetsRefs|GetBleedingScreen
      (:then
        (Utilities|MHIsWidgetVisible (Variables|WidgetsRefs|GetBleedingScreen)
          (:false
            (UserInterface|Viewport|AddtoViewport (Variables|WidgetsRefs|GetBleedingScreen) 0))))
      (:else
        (bind _returnvalue (UserInterface|CreateWidget "/Game/RAD_HORDE/Blueprints/Widgets/Game/BP_W_Bleeding.BP_W_Bleeding_C" (Variables|Default|GetPlayerOwner)))
        (bind _output_get (Variables|WidgetsRefs|SetBleedingScreen _returnvalue))
        (UserInterface|Viewport|AddtoViewport _output_get 0)))
    (else
      (bind _bleedingscreen (Variables|WidgetsRefs|GetBleedingScreen)
        (:then
          (Widget|RemovefromParent _bleedingscreen))
        (:else)))))

(fn FToggleObserverHud
  (params (Show :type Boolean))
  (if Show
    (Variables|WidgetsRefs|GetObserverHud
      (:then
        (Utilities|MHIsWidgetVisible (Variables|WidgetsRefs|GetObserverHud)
          (:false
            (UserInterface|Viewport|AddtoViewport (Variables|WidgetsRefs|GetObserverHud) 0))))
      (:else
        (bind _returnvalue (UserInterface|CreateWidget "/Game/RAD_HORDE/Blueprints/Widgets/Game/BP_W_ObserverHud.BP_W_ObserverHud_C" (Variables|Default|GetPlayerOwner)))
        (bind _output_get (Variables|WidgetsRefs|SetObserverHud _returnvalue))
        (UserInterface|Viewport|AddtoViewport _output_get 0)))
    (else
      (bind _observerhud (Variables|WidgetsRefs|GetObserverHud)
        (:then
          (Widget|RemovefromParent _observerhud))
        (:else)))))