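; Game State for the wave-based zombie horde mode, running the match cycle from lobby through repeating waves to finish and restart.
; On the server, setting GlobalState fires its RepNotify, which multicasts the change to event dispatchers and restarts a one-second countdown that advances the state.
; The lobby countdown waits for minimum players and shortens when all are ready, while waves end early once all zombies die.
; Multicasts also relay chat and kill feed updates.
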(event Custom|MC_OnGlobalStateChange
  (params (NewGlobalState :type E_GlobalState%20Enum :default "NewEnumerator23"))
  ;[1 0 0.3256] Multicast current state -> call event dispatcher on clients
  (switch Utilities|FlowControl|Switch|SwitchonE_GlobalState NewGlobalState
    (:NewEnumerator23
      (Default|CallDGameStartDelay))
    (:NewEnumerator0
      (Default|CallDLobbyState))
    (:NewEnumerator29
      (Default|CallDMatchStart))
    (:NewEnumerator28
      (Default|CallDBeforeWave))
    (:NewEnumerator17
      (Default|CallDPlayTime))
    (:NewEnumerator30
      (Default|CallDAfterWave))
    (:NewEnumerator26
      (Default|CallDMatchFinish))))

(event Custom|EA_FinishPlayTime
  ;[1 1 1] Finish wave
  (Kernel|FSDefineNextGlobalState))

(event Custom|MC_UpdateKillFeed
  (params (PlayerId :type Integer) (WeaponId :type Integer) (IsHeadShot :type Boolean))
  ;[0 0.8706 1] Update kills log
  (Default|CallDUpdateKillFeed PlayerId WeaponId IsHeadShot))

(event Custom|EA_OnZombieDeath
  ;[1 1 1] Finish wave on last zombie death
  (if (Info|FSCanFinishWaveonZombieDeath)
    (CallFunction|EAFinishPlayTime)))

(event Custom|MC_UpdateGameChat
  (params (IsServer :type Boolean) (SenderId :type Integer) (Message :type String))
  ;[0 0.8706 1] Update game chat
  (Default|CallDUpdateGameChat IsServer SenderId Message))

(event Custom|EA_FinishMatch
  ;[1 1 1] Finish match
  (Utilities|FlowControl|Delay 2.0)
  (Variables|CurrentState|SetGlobalState "NewEnumerator26"))

(event Custom|MC_UpdateLobbyChat
  (params (PlayerId :type Integer) (Message :type String))
  ;[0 0.8706 1] Update lobby chat
  (Default|CallDUpdateLobbyChat PlayerId Message))

(event EventBeginPlay
  ;[1 0.7631 0] BEGIN PLAY
  (Networking|SwitchHasAuthority
    (:Authority
      ;;[1 0 0] It starts main timer. OnRep_GlobalState.
      (Variables|CurrentState|SetGlobalState "NewEnumerator23"))))

(fn ConstructionScript)

(fn FGetTotalPlayers
  (return (Utilities|Array|Length (Variables|Default|GetPlayerArray))))

(fn FGetTotalAlivePlayers
  (LocalVariables|SetAlivePlayers_L 0)
  (for _array_element (Variables|Default|GetPlayerArray)
    (bind _asbp_kernel_ps (Utilities|Casting|CastToBP_Kernel_PS _array_element))
    (if (not (Variables|/Game/RAD_HORDE/Blueprints/Kernel/BP_Kernel_PS.BP_Kernel_PS_C|GetIsDead _asbp_kernel_ps))
      (LocalVariables|SetAlivePlayers_L (+ (LocalVariables|GetAlivePlayers_L) 1))))
  (return (LocalVariables|GetAlivePlayers_L)))

(fn FSDecreaseTime
  (bind _output_get (Variables|CurrentState|SetCurrentTime (- (Variables|CurrentState|GetCurrentTime) 1)))
  (return (<= _output_get 0)))

(fn FSMainTimer
  (switch Utilities|FlowControl|Switch|SwitchonE_GlobalState (Variables|CurrentState|GetGlobalState)
    (:NewEnumerator23
      (bind _istimeover (MainTimer|FSDecreaseTime :!label _label))
      (if _istimeover
        (MainTimer|FSStopMainTimer)
        (Kernel|FSDefineNextGlobalState)))
    (:NewEnumerator0
      ;[1 1 1] If there are not enought players do not update lobby time
      (if (>= (AlivePlayers|FGetTotalPlayers) (Variables|/Game/RAD_HORDE/Blueprints/Kernel/BP_Kernel_GM.BP_Kernel_GM_C|GetMinPlayersToStart (CallFunction|HKernelGM)))
        (goto _label)
        (else
          (Variables|CurrentState|SetCurrentTime (Variables|TimeSettings|GetLobbyTimeS)))))
    (:NewEnumerator29
      (goto _label))
    (:NewEnumerator28
      (goto _label))
    (:NewEnumerator17
      (goto _label))
    (:NewEnumerator30
      (goto _label))
    (:NewEnumerator26
      (goto _label))))

(fn FSStartMainTimer
  (params (NewTime :type Integer))
  (Networking|SwitchHasAuthority
    (:Authority
      (MainTimer|FSStopMainTimer)
      (Variables|CurrentState|SetCurrentTime NewTime)
      (bind _returnvalue (Utilities|Time|SetTimerbyFunctionName 0 "FS_MainTimer" 1.0 true))
      (Variables|Timers|SetMainTimer _returnvalue))))

(fn FSStopMainTimer
  (params (NewParam :type Integer))
  (Utilities|Time|ClearandInvalidateTimerbyHandle (Variables|Timers|GetMainTimer)))

(fn OnRepGlobalState
  (Networking|SwitchHasAuthority
    (:Authority
      (MainTimer|FSStopMainTimer)
      (CallFunction|MConGlobalStateChange (Variables|CurrentState|GetGlobalState))
      (switch Utilities|FlowControl|Switch|SwitchonE_GlobalState (Variables|CurrentState|GetGlobalState)
        (:NewEnumerator23
          (MainTimer|FSStartMainTimer (Variables|TimeSettings|GetGameStartDelayS)))
        (:NewEnumerator0
          (MainTimer|FSStartMainTimer (Variables|TimeSettings|GetLobbyTimeS)))
        (:NewEnumerator29
          (MainTimer|FSStartMainTimer (Variables|TimeSettings|GetMatchStartTimeS)))
        (:NewEnumerator28
          (MainTimer|FSStartMainTimer (Variables|TimeSettings|GetBeforeWaveTimeS)))
        (:NewEnumerator17
          (MainTimer|FSStartMainTimer (Variables|TimeSettings|GetPlayTimeS)))
        (:NewEnumerator30
          (MainTimer|FSStartMainTimer (Variables|TimeSettings|GetAfterWaveTimeS)))
        (:NewEnumerator26
          (MainTimer|FSStartMainTimer (Variables|TimeSettings|GetMatchFinishTimeS)))))))

(fn FSDefineNextGlobalState
  (switch Utilities|FlowControl|Switch|SwitchonE_GlobalState (Variables|CurrentState|GetGlobalState)
    (:NewEnumerator23
      (Variables|CurrentState|SetCurrentWave 0)
      (Variables|CurrentState|SetGlobalState "NewEnumerator0"))
    (:NewEnumerator0
      (Variables|CurrentState|SetGlobalState "NewEnumerator29"))
    (:NewEnumerator29
      (Variables|CurrentState|SetGlobalState "NewEnumerator28"))
    (:NewEnumerator28
      (Variables|CurrentState|SetCurrentWave (+ (Variables|CurrentState|GetCurrentWave) 1))
      (Variables|CurrentState|SetGlobalState "NewEnumerator17"))
    (:NewEnumerator17
      (Variables|CurrentState|SetGlobalState "NewEnumerator30"))
    (:NewEnumerator30
      (if (Info|FSIsLastWave)
        (Variables|CurrentState|SetGlobalState "NewEnumerator26")
        (else
          (Variables|CurrentState|SetGlobalState "NewEnumerator28"))))
    (:NewEnumerator26
      (Variables|CurrentState|SetGlobalState "NewEnumerator23"))))

(fn FFindLastAlivePlayer
  (for _array_element (Variables|Default|GetPlayerArray)
    (bind _asbp_kernel_ps (Utilities|Casting|CastToBP_Kernel_PS _array_element))
    (if (not (Variables|/Game/RAD_HORDE/Blueprints/Kernel/BP_Kernel_PS.BP_Kernel_PS_C|GetIsDead _asbp_kernel_ps))
      (return _array_element))))

(fn FSIsLastWave
  (return (>= (Variables|CurrentState|GetCurrentWave) (Variables|/Game/RAD_HORDE/Blueprints/Kernel/BP_Kernel_GM.BP_Kernel_GM_C|GetTotalWaves (CallFunction|HKernelGM)))))

(fn FSTrytoStartLobbyCountdown
  (for _array_element (Variables|Default|GetPlayerArray)
    (bind _asbp_kernel_ps (Utilities|Casting|CastToBP_Kernel_PS _array_element))
    (if (not (Variables|/Game/RAD_HORDE/Blueprints/Kernel/BP_Kernel_PS.BP_Kernel_PS_C|GetIsReady _asbp_kernel_ps))
      (return)))
  (if (and (Utilities|Enum|Equal(Enum) (Variables|CurrentState|GetGlobalState) "NewEnumerator0") (> (Variables|CurrentState|GetCurrentTime) 5))
    (Variables|CurrentState|SetCurrentTime 5)))

(fn FSCanFinishWaveonZombieDeath
  (LocalVariables|SetFinishWave_L true)
  (bind _outactors (Actor|GetAllActorsOfClass "/Game/RAD_HORDE/Blueprints/Zombie/Alpha_zombie/BP_Alpha.BP_Alpha_C"))
  (for _array_element _outactors
    (if (not (Variables|/Game/RAD_HORDE/Blueprints/Zombie/Alpha_zombie/BP_Alpha.BP_Alpha_C|GetIsDead _array_element))
      (LocalVariables|SetFinishWave_L false)))
  (return (LocalVariables|GetFinishWave_L)))