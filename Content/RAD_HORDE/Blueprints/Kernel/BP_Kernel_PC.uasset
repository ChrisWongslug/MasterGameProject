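; Base "Kernel" player controller for the multiplayer horde mode, handling session, lobby, chat and UI input.
; On begin play it pulls host settings from the GameMode by server RPC and caches them in the local GameInstance for UI.
; Server RPCs relay chat, ready status and pawn destruction, while keys toggle HUD panels.
; Team interface calls forward to PlayerState, and a test key shortens the GameState timer.
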(event Custom|CL_SaveHostSettingsInLocalGI
  (params (ServerName :type String) (MapId :type Integer) (MaxPlayers :type Integer) (MinPlayerToStart :type Integer) (TotalWaves :type Integer))
  (bind _maingi (CallFunction|HMainGI))
  ;[1 0 0.1247] Save host settings in local GameInstance. We need them for UI
  (Variables|/Game/RAD_HORDE/Blueprints/Kernel/BP_MainGI.BP_MainGI_C|SetServerName _maingi ServerName)
  (Variables|/Game/RAD_HORDE/Blueprints/Kernel/BP_MainGI.BP_MainGI_C|SetMapId _maingi MapId)
  (Variables|/Game/RAD_HORDE/Blueprints/Kernel/BP_MainGI.BP_MainGI_C|SetMaxPlayers _maingi MaxPlayers)
  (Variables|/Game/RAD_HORDE/Blueprints/Kernel/BP_MainGI.BP_MainGI_C|SetMinPlayerToStart _maingi MinPlayerToStart)
  (Variables|/Game/RAD_HORDE/Blueprints/Kernel/BP_MainGI.BP_MainGI_C|SetTotalWaves _maingi TotalWaves))

(event Custom|SRV_GetHostSettings
  (bind _kernelgm (CallFunction|HKernelGM))
  ;[1 0 0.1247] Get host settings from server
  (CallFunction|CLSaveHostSettingsinLocalGI (Variables|/Game/RAD_HORDE/Blueprints/Kernel/BP_Kernel_GM.BP_Kernel_GM_C|GetServerName _kernelgm) (Variables|/Game/RAD_HORDE/Blueprints/Kernel/BP_Kernel_GM.BP_Kernel_GM_C|GetMapId _kernelgm) (Variables|/Game/RAD_HORDE/Blueprints/Kernel/BP_Kernel_GM.BP_Kernel_GM_C|GetMaxPlayers _kernelgm) (Variables|/Game/RAD_HORDE/Blueprints/Kernel/BP_Kernel_GM.BP_Kernel_GM_C|GetMinPlayersToStart _kernelgm) (Variables|/Game/RAD_HORDE/Blueprints/Kernel/BP_Kernel_GM.BP_Kernel_GM_C|GetTotalWaves _kernelgm)))

(event Custom|SRV_DestroyPawn
  (bind _returnvalue (Pawn|GetSpectatorPawn))
  ;[1 1 1] Destroy character
  (Utilities|IsValid _returnvalue
    (:Is%20Valid
      (Actor|DestroyActor _returnvalue))
    (:Is%20Not%20Valid
      _))
  (Class|BPICharacter|IEDestroySelf(Message) (Pawn|GetControlledPawn)))

(event Custom|CL_Disconnect
  ;[1 1 1] Disconnect
  (Game|OpenLevel(byName) "MainMenu")
  (|DestroySession self))

(event Custom|srv_5
  ;[1 1 1] for testing. set current time = 2 seconds
  (Variables|/Game/RAD_HORDE/Blueprints/Kernel/BP_Kernel_GS.BP_Kernel_GS_C|SetCurrentTime (CallFunction|HKernelGS) 2))

(event EventEndPlay
  (params (EndPlayReason :type EEndPlayReason%20Enum :default "Destroyed"))
  ;[1 1 1] Disconnect
  (CallFunction|IEDestroyControlledPawn))

(event EventIEDestroyControlledPawn
  ;[1 1 1] Destroy character
  (CallFunction|SRVDestroyPawn))

(event EventIEDisconnectfromtheServer
  ;[1 1 1] Disconnect
  (CallFunction|IEDestroyControlledPawn)
  (CallFunction|CLDisconnect))

(event EventBeginPlay
  ;[1 1 1] Begin play. Load game setting from server - we need them for ui
  (if (Pawn|IsLocalPlayerController)
    (CallFunction|SRVGetHostSettings)))

(event Input|KeyboardEvents|Add
  (params (Key :type Key%20Structure))
  ;[1 1 1] for testing. set current time = 2 seconds
  (:Pressed
    (CallFunction|Srv5)))

(event Custom|SRV_SendChatMessage
  (params (IsServer :type Boolean) (Message :type String))
  ;[0 0.6122 1] Send chat message
  (Default|MCUpdateGameChat (CallFunction|HKernelGS) IsServer (Variables|/Script/Engine.PlayerState|GetPlayerId (Variables|GetPlayerState)) Message))

(event Custom|SRV_ChangeReadyStatus
  (params (IsReady :type Boolean))
  ;[1 1 1] Change ready status in lobby
  (bind _asbp_kernel_ps (Utilities|Casting|CastToBP_Kernel_PS (Variables|GetPlayerState)))
  (Variables|/Game/RAD_HORDE/Blueprints/Kernel/BP_Kernel_PS.BP_Kernel_PS_C|SetIsReady _asbp_kernel_ps IsReady)
  (Default|FSTrytoStartLobbyCountdown (CallFunction|HKernelGS)))

(event Custom|SRV_SendLobbyMessage
  (params (Message :type String))
  ;[1 1 1] Send lobby message
  (Default|MCUpdateLobbyChat (CallFunction|HKernelGS) (Variables|/Script/Engine.PlayerState|GetPlayerId (Variables|GetPlayerState)) Message))

(event Input|KeyboardEvents|Z
  (params (Key :type Key%20Structure))
  (bind _kernelhud (CallFunction|HKernelHUD))
  (bind _returnvalue (Game|GetPlayerCharacter 0))
  (bind _returnvalue_2 (Game|GetPlayerCharacter 0))
  (bind _lobby (Variables|/Game/RAD_HORDE/Blueprints/Kernel/BP_Kernel_HUD.BP_Kernel_HUD_C|GetLobby _kernelhud))
  ;[1 1 1] Show / hide in-game menu
  (:Pressed
    (bind _isa (Utilities|FlowControl|FlipFlop)
      (:A
        (if _isa
          (Default|FToggleinGameMenu (CallFunction|HKernelHUD) true)
          (Variables|Default|SetbShowMouseCursor true)
          (Utilities|IsValid _returnvalue_2
            (:Is%20Valid
              (Input|DisableInput _returnvalue_2 self)))))
      (:B
        (Default|FToggleinGameMenu (CallFunction|HKernelHUD) false)
        (Utilities|FlowControl|Sequence
          (:then_0
            (Variables|/Script/Engine.PlayerController|SetbShowMouseCursor (Game|GetPlayerController 0) false)
            (Utilities|IsValid _returnvalue
              (:Is%20Valid
                (Input|EnableInput _returnvalue self))))
          (:then_1
            (Utilities|IsValid _lobby
              (:Is%20Valid
                (if (Widget|IsVisible _lobby)
                  (Variables|/Script/Engine.PlayerController|SetbShowMouseCursor (Game|GetPlayerController 0) true))))))))))

(event Input|KeyboardEvents|Tab
  (params (Key :type Key%20Structure))
  (bind _kernelhud (CallFunction|HKernelHUD))
  ;[1 1 1] Toggle scoreboard
  (:Pressed
    (Default|FToggleGameChat _kernelhud false)
    (Default|FToggleScoreboard _kernelhud true))
  (:Released
    (Default|FToggleScoreboard _kernelhud false)))

(event Input|KeyboardEvents|Q
  (params (Key :type Key%20Structure))
  (bind _kernelhud (CallFunction|HKernelHUD))
  ;[1 1 1] Toggle help
  (:Pressed
    (Default|FToggleGameChat _kernelhud false)
    (Default|FToggleHelp _kernelhud true))
  (:Released
    (Default|FToggleHelp _kernelhud false)))

(event Input|KeyboardEvents|Enter
  (params (Key :type Key%20Structure))
  (bind _kernelhud (CallFunction|HKernelHUD))
  ;[0 0.6122 1] Open game chat
  (:Pressed
    (switch Utilities|FlowControl|Switch|SwitchonE_GlobalState (Variables|/Game/RAD_HORDE/Blueprints/Kernel/BP_Kernel_GS.BP_Kernel_GS_C|GetGlobalState (CallFunction|HKernelGS))
      (:NewEnumerator29
        _)
      (:NewEnumerator28
        _)
      (:NewEnumerator17
        _)
      (:NewEnumerator30
        _))
    (Default|FToggleGameChat _kernelhud true)
    (Default|EOpenChat (Variables|/Game/RAD_HORDE/Blueprints/Kernel/BP_Kernel_HUD.BP_Kernel_HUD_C|GetGameChat _kernelhud))))

(event Input|KeyboardEvents|Escape
  (params (Key :type Key%20Structure))
  (bind _kernelhud (CallFunction|HKernelHUD))
  (bind _returnvalue (Game|GetPlayerCharacter 0))
  (bind _returnvalue_2 (Game|GetPlayerCharacter 0))
  (bind _lobby (Variables|/Game/RAD_HORDE/Blueprints/Kernel/BP_Kernel_HUD.BP_Kernel_HUD_C|GetLobby _kernelhud))
  ;[1 1 1] Show / hide in-game menu
  (:Pressed
    (bind _isa (Utilities|FlowControl|FlipFlop)
      (:A
        (if _isa
          (Default|FToggleinGameMenu (CallFunction|HKernelHUD) true)
          (Variables|Default|SetbShowMouseCursor true)
          (Utilities|IsValid _returnvalue_2
            (:Is%20Valid
              (Input|DisableInput _returnvalue_2 self)))))
      (:B
        (Default|FToggleinGameMenu (CallFunction|HKernelHUD) false)
        (Utilities|FlowControl|Sequence
          (:then_0
            (Variables|/Script/Engine.PlayerController|SetbShowMouseCursor (Game|GetPlayerController 0) false)
            (Utilities|IsValid _returnvalue
              (:Is%20Valid
                (Input|EnableInput _returnvalue self))))
          (:then_1
            (Utilities|IsValid _lobby
              (:Is%20Valid
                (if (Widget|IsVisible _lobby)
                  (Variables|/Script/Engine.PlayerController|SetbShowMouseCursor (Game|GetPlayerController 0) true))))))))))

(fn ConstructionScript)

(fn IFGetTeam
  (bind _team (Class|BPITeamPlayer|IFGetTeam(Message) (Variables|GetPlayerState)))
  (return _team))

(fn IFSetTeam
  (params (NewTeam :type Integer))
  (bind _team (Class|BPITeamPlayer|IFSetTeam(Message) (Variables|GetPlayerState) NewTeam))
  (return _team))