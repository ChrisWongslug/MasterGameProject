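; Kernel game mode for the wave-based horde game, managing server settings, player connections and pawn spawning.
; Settings load once from the game instance or dedicated-server command line, triggered from BeginPlay and PostLogin because login can precede BeginPlay.
; Login tracks players and rejects extras when the server is full; logout removes them and their pawns.
; Game state match dispatchers trigger spawning at random spawn points on start and delayed pawn destruction on finish.
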(event Custom|E_InitSettings
  ;[1 0.5159 0.0913] INIT SETTINGS
  (if (not (Variables|Config|GetWasInitSettingsSet))
    (Utilities|FlowControl|Sequence
      (:then_0
        (if (Networking|IsDedicatedServer)
          (InitSettings|FSSetGameModeSettingsforDedicatedServer)
          (else
            ;;[1 1 1 1 15] Get host game settings from MainGI
            (InitSettings|FSSetHostGameSettings)))
        ;;[1 1 1] Check and set some default values to avoid errors
        (InitSettings|FCheckHostSettings))
      (:then_1
        (Variables|Config|SetWasInitSettingsSet true)))))

(event Custom|EA_StartMatch
  ;[1 0 0] Spawn players at match start
  (PlayerRespawn|FSSpawnAllPlayers))

(event Custom|E_FinishMatch
  ;[1 0 0] Match finish - destroy all pawns
  (Utilities|FlowControl|Delay 0.5)
  (Players|FSDestroyAllPlayers))

(event EventBeginPlay
  ;[1 0 0] BEGIN PLAY
  (Utilities|FlowControl|Sequence
    (:then_0
      (Utilities|IsValid (CallFunction|HKernelGS)
        (:Is%20Valid
          _)
        (:Is%20Not%20Valid
          (Utilities|FlowControl|Delay 0.2)))
      (Utilities|FlowControl|Sequence
        (:then_0
          ;[1 0 0] Spawn players at match start
          (EventDispatchers|BindEventtoDMatchStart (CallFunction|HKernelGS) (delegate Custom|EA_StartMatch)))
        (:then_1
          ;[1 0 0] Match finish - destroy all pawns
          (EventDispatchers|BindEventtoDMatchFinish (CallFunction|HKernelGS) (delegate Custom|E_FinishMatch)))))
    (:then_1
      (CallFunction|EInitSettings))))

(event EventPostLogin
  (params (NewPlayer :type Player%20Controller%20Object%20Reference))
  ;[0 0.1238 1] LogIn event.
  ; Since OnPostLogin event can be called before BeginPlay event (issue UE-27284), I set "init settings" also in OnPostLogin event to be sure all settings was set right
  (Utilities|FlowControl|Sequence
    (:then_0
      (CallFunction|EInitSettings))
    (:then_1
      (NewPlayersProcessing|FSonPostLogin NewPlayer))))

(event EventOnLogout
  (params (ExitingController :type Controller%20Object%20Reference))
  ;[0 0.1238 1] LogOut event. Update session info
  (CallFunction|FSonLogout ExitingController))

(fn ConstructionScript)

(fn FSonLogout
  (params (ExitingController :type Controller%20Object%20Reference))
  (bind _asplayer_controller (Utilities|Casting|CastToPlayerController ExitingController))
  (LocalVariables|SetExitingPCLocal _asplayer_controller)
  (Utilities|FlowControl|Sequence
    (:then_0
      (Utilities|IsValid (Pawn|GetControlledPawn (LocalVariables|GetExitingPCLocal))
        (:Is%20Valid
          (Class|BPICharacter|IEDestroySelf(Message) (Pawn|GetControlledPawn (LocalVariables|GetExitingPCLocal))))))
    (:then_1
      (Utilities|Array|RemoveItem (Variables|Players|GetConnectedPlayers) (LocalVariables|GetExitingPCLocal))
      (LocalVariables|SetExitingPCLocal 0))))

(fn FSonPostLogin
  (params (NewPC :type Player%20Controller%20Object%20Reference))
  (bind _output_get (LocalVariables|SetNewPC_L NewPC))
  (Utilities|FlowControl|Sequence
    (:then_0
      ;[1 1 1] disconnect new player if there is already maximim players on the server
      (if (Info|FSShouldDisconnectNewPlayer)
        (Class|BPIBasePlayerController|IEDisconnectfromtheServer(Message) (LocalVariables|GetNewPC_L))
        (return)))
    (:then_1
      (Utilities|Array|AddUnique (Variables|Players|GetConnectedPlayers) _output_get))))

(fn FSSpawnAllPlayers
  (for _array_element (Variables|Players|GetConnectedPlayers)
    (PlayerRespawn|FSSpawnPlayer _array_element (PlayerRespawn|FSGetSpawnLocation))))

(fn FSDestroyAllPlayers
  (for _array_element (Variables|Players|GetConnectedPlayers)
    (Class|BPIBasePlayerController|IEDestroyControlledPawn(Message) _array_element)))

(fn FSSpawnPlayer
  (params (PC :type Player%20Controller%20Object%20Reference) (RespawnLocation :type Transform))
  (bind _output_get (LocalVariables|SetPC_L PC))
  (Class|BPIBasePlayerController|IEDestroyControlledPawn(Message) _output_get)
  (bind _returnvalue (Game|SpawnActorfromClass (Variables|Config|GetPawnClass) RespawnLocation "AdjustIfPossibleButAlwaysSpawn" (LocalVariables|GetPC_L) 0))
  (Utilities|IsValid _returnvalue
    (:Is%20Valid
      (Pawn|Possess (LocalVariables|GetPC_L) _returnvalue)
      (return _returnvalue))
    (:Is%20Not%20Valid
      (Development|PrintString "RESPAWN ERROR" true true "(R=1.000000,G=0.000000,B=0.000000,A=1.000000)" 22.0))))

(fn FSSetHostGameSettings
  (bind _maingi (CallFunction|HMainGI))
  (Variables|HostSettings|SetServerName (Variables|/Game/RAD_HORDE/Blueprints/Kernel/BP_MainGI.BP_MainGI_C|GetServerName _maingi))
  (Variables|HostSettings|SetMapId (Variables|/Game/RAD_HORDE/Blueprints/Kernel/BP_MainGI.BP_MainGI_C|GetMapId _maingi))
  (Variables|HostSettings|SetMaxPlayers (Variables|/Game/RAD_HORDE/Blueprints/Kernel/BP_MainGI.BP_MainGI_C|GetMaxPlayers _maingi))
  (Variables|HostSettings|SetMinPlayersToStart (Variables|/Game/RAD_HORDE/Blueprints/Kernel/BP_MainGI.BP_MainGI_C|GetMinPlayerToStart _maingi))
  (Variables|HostSettings|SetTotalWaves (Variables|/Game/RAD_HORDE/Blueprints/Kernel/BP_MainGI.BP_MainGI_C|GetTotalWaves _maingi)))

(fn FSSetGameModeSettingsforDedicatedServer
  (bind _returnvalue (Utilities|GetCommandLine))
  (LocalVariables|SetCommandLine _returnvalue)
  (Utilities|FlowControl|Sequence
    (:then_0
      ;[1 1 1] server name
      (Variables|HostSettings|SetServerName (CallFunction|HParseOption (LocalVariables|GetCommandLine) "sn")))
    (:then_1
      ;[1 1 1] map id
      (bind _returnvalue_2 (Game|GetCurrentLevelName true))
      (switch string _returnvalue_2
        (:ExampleMap
          (Variables|HostSettings|SetMapId 1))
        (:TestMap
          (Variables|HostSettings|SetMapId 2))))
    (:then_2
      ;[1 1 1] min players to start
      (Variables|HostSettings|SetMinPlayersToStart (Math|Conversions|ToInteger(Byte) (CallFunction|HParseOption (LocalVariables|GetCommandLine) "ms"))))
    (:then_3
      ;[1 1 1] max players
      (Variables|HostSettings|SetMaxPlayers (Math|Conversions|ToInteger(Byte) (CallFunction|HParseOption (LocalVariables|GetCommandLine) "mp"))))
    (:then_4
      ;[1 1 1] Total waves
      (Variables|HostSettings|SetTotalWaves (Math|Conversions|ToInteger(Byte) (CallFunction|HParseOption (LocalVariables|GetCommandLine) "tw"))))))

(fn FCheckHostSettings
  (Utilities|FlowControl|Sequence
    (:then_0
      (Utilities|MHIsEmptyString (Variables|HostSettings|GetServerName)
        (:true
          (Variables|HostSettings|SetServerName "Unnamed Server"))))
    (:then_1
      (if (== (Variables|HostSettings|GetMaxPlayers) 0)
        (Variables|HostSettings|SetMaxPlayers 4)))
    (:then_2
      (if (or (<= (Variables|HostSettings|GetMinPlayersToStart) 0) (> (Variables|HostSettings|GetMinPlayersToStart) 4))
        (Variables|HostSettings|SetMinPlayersToStart 1)))))

(fn FSShouldDisconnectNewPlayer
  (return (>= (Default|FGetTotalPlayers (CallFunction|HKernelGS)) (Variables|HostSettings|GetMaxPlayers))))

(fn FSGetSpawnLocation
  (bind _outactors (Actor|GetAllActorsOfClass "/Game/RAD_HORDE/Blueprints/Kernel/BP_SpawnPoint.BP_SpawnPoint_C"))
  (return (PlayerRespawn|FSGetRandomLocation _outactors)))

(fn FSGetRandomLocation
  (params (SpawnPoints :type Array%20of%20BP%20Spawn%20Point%20Object%20References))
  (bind _returnvalue (Utilities|Array|Length SpawnPoints))
  (bind _returnvalue_2 (- _returnvalue 1))
  (bind _returnvalue_3 (Math|Random|RandomInteger _returnvalue_2))
  (bind _output (Utilities|Array|Get(acopy) SpawnPoints _returnvalue_3))
  (Utilities|IsValid _output
    (:Is%20Valid
      (return (Transformation|GetActorTransform _output)))
    (:Is%20Not%20Valid
      (return (Math|Transform|MakeTransform "0, 0, 0")))))