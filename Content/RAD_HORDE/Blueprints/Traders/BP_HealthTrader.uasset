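; BP_HealthTrader is an interactable trader that sells a full heal to the player.
; It is always focusable and shows a "HEAL UP" prompt.
; On interact, it reads Money and Health from the character's BP_Kernel_PS player state, requiring enough for Price and health below full.
; It then sends a set-health interface message to the character and deducts Price directly from the player state's Money.
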(event EventIEInteract
  (params (Character :type Character%20Object%20Reference))
  (bind _asbp_base_character (Utilities|Casting|CastToBP_BaseCharacter Character))
  (bind _asbp_kernel_ps (Utilities|Casting|CastToBP_Kernel_PS (Variables|/Script/Engine.Pawn|GetPlayerState _asbp_base_character)))
  (if (and (>= (Variables|/Game/RAD_HORDE/Blueprints/Kernel/BP_Kernel_PS.BP_Kernel_PS_C|GetMoney _asbp_kernel_ps) (Variables|Default|GetPrice)) (< (Variables|/Game/RAD_HORDE/Blueprints/Kernel/BP_Kernel_PS.BP_Kernel_PS_C|GetHealth _asbp_kernel_ps) 1e+02))
    (Class|BPICharacter|IFSetHealth(Message) _asbp_base_character 1e+02)
    (Variables|/Game/RAD_HORDE/Blueprints/Kernel/BP_Kernel_PS.BP_Kernel_PS_C|SetMoney _asbp_kernel_ps (- (Variables|/Game/RAD_HORDE/Blueprints/Kernel/BP_Kernel_PS.BP_Kernel_PS_C|GetMoney _asbp_kernel_ps) (Variables|Default|GetPrice)))))

(fn ConstructionScript)

(fn IFCanFocus
  (return true))

(fn IFGetFocusMessage
  (return "HEAL UP"))