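; BP_AmmoTrader is an interactable trader that sells ammo to players, showing a "BUY AMMO" focus prompt.
; On interact, it checks the character's BP_Kernel_PS Money against Price.
; If affordable, it adds a fixed amount of ammo to the primary and secondary firearms in the weapons manager, then deducts Price.
; The charge runs as its own sequence step, so it applies even when no weapon receives ammo.
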(event EventIEInteract
  (params (Character :type Character%20Object%20Reference))
  (bind _asbp_base_character (Utilities|Casting|CastToBP_BaseCharacter Character))
  (bind _asbp_kernel_ps (Utilities|Casting|CastToBP_Kernel_PS (Variables|/Script/Engine.Pawn|GetPlayerState _asbp_base_character)))
  (if (>= (Variables|/Game/RAD_HORDE/Blueprints/Kernel/BP_Kernel_PS.BP_Kernel_PS_C|GetMoney _asbp_kernel_ps) (Variables|Default|GetPrice))
    (Utilities|FlowControl|Sequence
      (:then_0
        (Utilities|IsValid (Variables|/Game/RAD_HORDE/Blueprints/Characters/BP_WeaponsManager.BP_WeaponsManager_C|GetPrimaryWeapon (Variables|/Game/RAD_HORDE/Blueprints/Characters/BP_BaseCharacter.BP_BaseCharacter_C|GetBP_WeaponsManager _asbp_base_character))
          (:Is%20Valid
            (bind _asbp_firearm_weapon (Utilities|Casting|CastToBP_FirearmWeapon (Variables|/Game/RAD_HORDE/Blueprints/Characters/BP_WeaponsManager.BP_WeaponsManager_C|GetPrimaryWeapon (Variables|/Game/RAD_HORDE/Blueprints/Characters/BP_BaseCharacter.BP_BaseCharacter_C|GetBP_WeaponsManager _asbp_base_character))))
            (Variables|/Game/RAD_HORDE/Blueprints/Weapons/BP_FirearmWeapon.BP_FirearmWeapon_C|SetAmmo _asbp_firearm_weapon (+ (Variables|/Game/RAD_HORDE/Blueprints/Weapons/BP_FirearmWeapon.BP_FirearmWeapon_C|GetAmmo _asbp_firearm_weapon) 100)))))
      (:then_1
        (Utilities|IsValid (Variables|/Game/RAD_HORDE/Blueprints/Characters/BP_WeaponsManager.BP_WeaponsManager_C|GetSecondaryWeapon (Variables|/Game/RAD_HORDE/Blueprints/Characters/BP_BaseCharacter.BP_BaseCharacter_C|GetBP_WeaponsManager _asbp_base_character))
          (:Is%20Valid
            (bind _asbp_firearm_weapon_2 (Utilities|Casting|CastToBP_FirearmWeapon (Variables|/Game/RAD_HORDE/Blueprints/Characters/BP_WeaponsManager.BP_WeaponsManager_C|GetSecondaryWeapon (Variables|/Game/RAD_HORDE/Blueprints/Characters/BP_BaseCharacter.BP_BaseCharacter_C|GetBP_WeaponsManager _asbp_base_character))))
            (Variables|/Game/RAD_HORDE/Blueprints/Weapons/BP_FirearmWeapon.BP_FirearmWeapon_C|SetAmmo _asbp_firearm_weapon_2 (+ (Variables|/Game/RAD_HORDE/Blueprints/Weapons/BP_FirearmWeapon.BP_FirearmWeapon_C|GetAmmo _asbp_firearm_weapon_2) 100)))))
      (:then_2
        (Variables|/Game/RAD_HORDE/Blueprints/Kernel/BP_Kernel_PS.BP_Kernel_PS_C|SetMoney _asbp_kernel_ps (- (Variables|/Game/RAD_HORDE/Blueprints/Kernel/BP_Kernel_PS.BP_Kernel_PS_C|GetMoney _asbp_kernel_ps) (Variables|Default|GetPrice)))))))

(fn ConstructionScript)

(fn IFCanFocus
  (return true))

(fn IFGetFocusMessage
  (return "BUY AMMO"))