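; BP_Gate is a sci-fi gate whose two door meshes slide open when a Character enters its Box trigger.
; The Opendoor timeline drives the X relative location of both doors, with the left one using a value derived from the right's.
; On exit, a short delay rechecks the CharOnGate flag before reversing the timeline, so quick re-entry keeps the gate open.
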(event OnComponentBeginOverlap(Box)
  (params (OverlappedComponent :type Primitive%20Component%20Object%20Reference) (OtherActor :type Actor%20Object%20Reference) (OtherComp :type Primitive%20Component%20Object%20Reference) (OtherBodyIndex :type Integer) (bFromSweep :type Boolean) (SweepResult :type Hit%20Result%20Structure%20%28by%20ref%29))
  (Utilities|Casting|CastToCharacter OtherActor)
  (Variables|Default|SetCharOnGate true)
  (bind _movedoors (Timeline|Opendoor Play)
    (:Update
      (Transformation|SetRelativeLocation (Variables|Default|GetSM_Gate_DoorRight) (Math|Vector|MakeVector _movedoors 0.0 0.0) false false)
      (bind _result (Math|Float|NegateFloat _movedoors)
        (:%20%20
          (Transformation|SetRelativeLocation (Variables|Default|GetSM_Gate_DoorLeft) (Math|Vector|MakeVector _result 0.0 0.0) false false))))))

(event OnComponentEndOverlap(Box)
  (params (OverlappedComponent :type Primitive%20Component%20Object%20Reference) (OtherActor :type Actor%20Object%20Reference) (OtherComp :type Primitive%20Component%20Object%20Reference) (OtherBodyIndex :type Integer))
  (Utilities|Casting|CastToCharacter OtherActor)
  (Variables|Default|SetCharOnGate false)
  (Utilities|FlowControl|Delay 0.2)
  (if (not (Variables|Default|GetCharOnGate))
    (bind _movedoors (Timeline|Opendoor Reverse)
      (:Update
        (Transformation|SetRelativeLocation (Variables|Default|GetSM_Gate_DoorRight) (Math|Vector|MakeVector _movedoors 0.0 0.0) false false)
        (bind _result (Math|Float|NegateFloat _movedoors)
          (:%20%20
            (Transformation|SetRelativeLocation (Variables|Default|GetSM_Gate_DoorLeft) (Math|Vector|MakeVector _result 0.0 0.0) false false)))))))

(fn ConstructionScript)