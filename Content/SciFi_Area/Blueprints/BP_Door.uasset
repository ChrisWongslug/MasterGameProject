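; BP_Door is an automatic sliding door that opens while a Character is inside its Box trigger.
; BeginPlay caches the closed position and derives the open one by offsetting local X by MoveLenght.
; Entering the box plays the Doormove timeline, which linearly interpolates the Door between the two positions.
; Leaving waits briefly, then reverses the timeline only if the CharOnGate flag is still false.
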(event OnComponentBeginOverlap(Box)
  (params (OverlappedComponent :type Primitive%20Component%20Object%20Reference) (OtherActor :type Actor%20Object%20Reference) (OtherComp :type Primitive%20Component%20Object%20Reference) (OtherBodyIndex :type Integer) (bFromSweep :type Boolean) (SweepResult :type Hit%20Result%20Structure%20%28by%20ref%29))
  (Utilities|Casting|CastToCharacter OtherActor)
  (Variables|Default|SetCharOnGate true)
  (bind _newtrack_0 (Timeline|Doormove Play)
    (:Update
      (Transformation|SetRelativeLocation (Variables|Default|GetDoor) (Math|Interpolation|Ease "Linear" _newtrack_0 (Variables|Default|GetDoor_Start_Pos) (Variables|Default|GetDoor_End_Pos)) false false))))

(event OnComponentEndOverlap(Box)
  (params (OverlappedComponent :type Primitive%20Component%20Object%20Reference) (OtherActor :type Actor%20Object%20Reference) (OtherComp :type Primitive%20Component%20Object%20Reference) (OtherBodyIndex :type Integer))
  (Utilities|Casting|CastToCharacter OtherActor)
  (Variables|Default|SetCharOnGate false)
  (Utilities|FlowControl|Delay 0.2)
  (if (not (Variables|Default|GetCharOnGate))
    (bind _newtrack_0 (Timeline|Doormove Reverse)
      (:Update
        (Transformation|SetRelativeLocation (Variables|Default|GetDoor) (Math|Interpolation|Ease "Linear" _newtrack_0 (Variables|Default|GetDoor_Start_Pos) (Variables|Default|GetDoor_End_Pos)) false false)))))

(event EventBeginPlay
  (bind _output_get (Variables|Default|SetDoor_Start_Pos (Variables|/Script/Engine.SceneComponent|GetRelativeLocation (Variables|Default|GetDoor))))
  (Variables|Default|SetDoor_End_Pos (Math|Vector|MakeVector (- (.x _output_get) (Variables|Default|GetMove_Lenght)) (.y _output_get) (.z _output_get))))

(fn ConstructionScript)